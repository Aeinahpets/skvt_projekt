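; Base NPC Blueprint that drives its AI through a State Tree component, set up for sight-based player detection.
; When its PawnSensing component sees a pawn, it flags the player as seen and stores that pawn.
; It then sends an AI.SeenPlayer event to the State Tree, with no check that the pawn is actually the player.
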(event `self.PawnSensing.OnSeePawn`
  (params (Pawn :type "Pawn Object Reference"))
  (set `self.SeenPlayer` true)
  (set `self.SeenPawn` Pawn)
  (`StateTreeComponent.SendStateTreeEvent` (`self.StateTree`) (make `StateTreeEvent` (struct :`TagName` "AI.SeenPlayer"))))

(fn `UserConstructionScript`
  (`parent.UserConstructionScript`))